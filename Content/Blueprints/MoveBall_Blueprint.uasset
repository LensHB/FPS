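; Moving ball actor that travels back and forth along a horizontal diagonal while its Movement flag is set.
; Tick moves it along normalized Direction at Speed, scaled by delta time without sweep, while a latent Delay and FlipFlop reverse Direction about every three seconds.
; Hits toggle Movement, beginning an overlap stops it and ending one resumes it.
; An X-bounds reversal using B1 and B2 is disconnected and never runs.
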(event EventBeginPlay)

(event Collision|EventActorBeginOverlap
  (params (OtherActor :type Actor%20Object%20Reference))
  (Variables|Default|SetMovement (Variables|Default|GetFalse)))

(event EventTick
  (params (DeltaSeconds :type Float%20%28single-precision%29))
  (bind _staticmeshcomponent (Variables|Debug|GetStaticMeshComponent))
  (bind _returnvalue (Transformation|GetWorldTransform _staticmeshcomponent))
  (bind (_location _rotation _scale) (Math|Transform|BreakTransform _returnvalue))
  (if (Variables|Default|GetMovement)
    (Transformation|SetActorTransform (Math|Transform|MakeTransform (+ _location (* (Math|Vector|Normalize (Variables|Default|Getdirection)) (* (Utilities|Time|GetWorldDeltaSeconds) (Variables|Default|GetSpeed)))) _rotation _scale))
    ;[1 1 1] Direction changing
    (Utilities|FlowControl|Delay 3.0)
    (Utilities|FlowControl|FlipFlop
      (:A
        (Variables|Default|Setdirection "-10.000000,-10.000000, 0"))
      (:B
        (Variables|Default|Setdirection "10.000000,10.000000, 0")))))

(event Collision|EventActorEndOverlap
  (params (OtherActor :type Actor%20Object%20Reference))
  (Variables|Default|SetMovement (Variables|Default|GetTrue)))

(event Collision|EventHit
  (params (MyComp :type Primitive%20Component%20Object%20Reference) (Other :type Actor%20Object%20Reference) (OtherComp :type Primitive%20Component%20Object%20Reference) (bSelfMoved :type Boolean) (HitLocation :type Vector :default "0, 0, 0") (HitNormal :type Vector :default "0, 0, 0") (NormalImpulse :type Vector :default "0, 0, 0") (Hit :type Hit%20Result%20Structure%20%28by%20ref%29))
  (Utilities|FlowControl|FlipFlop
    (:A
      (Variables|Default|SetMovement (Variables|Default|GetFalse)))
    (:B
      (Variables|Default|SetMovement (Variables|Default|GetTrue)))))

(fn ConstructionScript)