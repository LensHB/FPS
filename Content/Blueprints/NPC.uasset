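; Enemy NPC that chases any Character it sees and breaks apart when it attacks or gets hit.
; PawnSensing drives AI MoveTo; on arrival within range it damages the target and destroys itself.
; Attack, mesh hit and RadialDamage events each swap the NPC for a spawned destructible-mesh actor aligned to it, then damage that actor's DestructibleComponent to fracture it.
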(event OnSeePawn(PawnSensing)
  (params (Pawn :type Pawn%20Object%20Reference))
  (bind _returnvalue (Transformation|GetActorTransform))
  (bind (_location _rotation _scale) (Math|Transform|BreakTransform _returnvalue))
  (bind (_roll _pitch _yaw) (Math|Rotator|BreakRotator _rotation))
  ;[1 1 1] Chasing
  (bind _ascharacter (Utilities|Casting|CastToCharacter Pawn))
  (AI|AIMoveTo self "0, 0, 0" _ascharacter 5.0 false
    (:OnSuccess
      (if (<= (Math|Vector|VectorLength (- (Transformation|GetActorLocation _ascharacter) _location)) 5e+02)
        (bind _returnvalue_2 (Game|SpawnActorfromClass "/Game/Blueprints/StaticMesh_DM_Blueprint.StaticMesh_DM_Blueprint_C" (Math|Transform|MakeTransform (- _location (Math|Vector|MakeVector 0.0 0.0 9e+01)) (Math|Rotator|MakeRotator _roll _pitch (- _yaw 9e+01)) _scale) "AlwaysSpawn" 0 0))
        (Game|Damage|ApplyDamage _ascharacter 1e+01 0 self)
        (Class|DestructibleComponent|ApplyDamage (Variables|/Script/ApexDestruction.DestructibleActor|GetDestructibleComponent _returnvalue_2) 3.1e+03 (+ (Transformation|GetActorLocation _returnvalue_2) "0, 0,90.000000") (Transformation|GetActorLocation _returnvalue_2) 0.0)
        (Actor|DestroyActor)))))

(event OnComponentHit(Mesh)
  (params (HitComponent :type Primitive%20Component%20Object%20Reference) (OtherActor :type Actor%20Object%20Reference) (OtherComp :type Primitive%20Component%20Object%20Reference) (NormalImpulse :type Vector :default "0, 0, 0") (Hit :type Hit%20Result%20Structure%20%28by%20ref%29))
  (bind _returnvalue (Transformation|GetActorTransform))
  (bind (_location _rotation _scale) (Math|Transform|BreakTransform _returnvalue))
  (bind (_roll _pitch _yaw) (Math|Rotator|BreakRotator _rotation))
  ;[1 1 1] Destory(shoot)
  (bind _returnvalue_2 (Game|SpawnActorfromClass "/Game/Blueprints/StaticMesh_DM_Blueprint.StaticMesh_DM_Blueprint_C" (Math|Transform|MakeTransform (- _location (Math|Vector|MakeVector 0.0 0.0 9e+01)) (Math|Rotator|MakeRotator _roll _pitch (- _yaw 9e+01)) _scale) "Undefined" 0 0))
  (Actor|DestroyActor)
  (Class|DestructibleComponent|ApplyRadiusDamage (Variables|/Script/ApexDestruction.DestructibleActor|GetDestructibleComponent _returnvalue_2) 5e+03 (.ImpactPoint (Collision|BreakHitResult Hit)) 5e+01 5e+03 true))

(event EventBeginPlay)

(event Game|Damage|EventRadialDamage
  (params (DamageReceived :type Float%20%28single-precision%29) (DamageType :type Damage%20Type%20Object%20Reference) (Origin :type Vector :default "0, 0, 0") (HitInfo :type Hit%20Result%20Structure%20%28by%20ref%29) (InstigatedBy :type Controller%20Object%20Reference) (DamageCauser :type Actor%20Object%20Reference))
  (bind _returnvalue (Transformation|GetActorTransform))
  (bind (_location _rotation _scale) (Math|Transform|BreakTransform _returnvalue))
  (bind (_roll _pitch _yaw) (Math|Rotator|BreakRotator _rotation))
  (bind _returnvalue_2 (Game|SpawnActorfromClass "/Game/Blueprints/StaticMesh_DM_Blueprint.StaticMesh_DM_Blueprint_C" (Math|Transform|MakeTransform (- _location (Math|Vector|MakeVector 0.0 0.0 9e+01)) (Math|Rotator|MakeRotator _roll _pitch (- _yaw 9e+01)) _scale) "Undefined" 0 0))
  (Actor|DestroyActor)
  (Class|DestructibleComponent|ApplyRadiusDamage (Variables|/Script/ApexDestruction.DestructibleActor|GetDestructibleComponent _returnvalue_2) 5e+03 (+ _location "0, 0,90.000000") 5e+01 5e+03 true))

(event EventTick
  (params (DeltaSeconds :type Float%20%28single-precision%29)))

(fn ConstructionScript)