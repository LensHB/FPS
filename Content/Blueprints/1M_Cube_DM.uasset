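; 1M_Cube_DM is a destructible actor that moves until it hits something, shatters, then loads the LV_Soul_Slum level.
; Tick offsets it along local Z by a fixed per-frame step, without sweep or delta-time scaling, until NewVar0 is set.
; The Destructible's hit event sets that flag, applies heavy damage at the impact point, and opens the level after a short delay.
; AnyDamage only prints a debug string.
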(event OnComponentHit(Destructible)
  (params (HitComponent :type Primitive%20Component%20Object%20Reference) (OtherActor :type Actor%20Object%20Reference) (OtherComp :type Primitive%20Component%20Object%20Reference) (NormalImpulse :type Vector :default "0, 0, 0") (Hit :type Hit%20Result%20Structure%20%28by%20ref%29))
  (bind (_bblockinghit _binitialoverlap _time _distance _location _impactpoint _normal _impactnormal) (Collision|BreakHitResult Hit))
  (Variables|Default|SetNewVar_0 (>= 1e+01 0.0))
  (Class|DestructibleComponent|ApplyDamage (Variables|Default|GetDestructible self) 1e+03 _impactpoint _impactnormal 0.0)
  (Utilities|FlowControl|Delay 3.0)
  (Game|OpenLevel(byName) "LV_Soul_Slum"))

(event EventBeginPlay)

(event Collision|EventActorBeginOverlap
  (params (OtherActor :type Actor%20Object%20Reference)))

(event EventTick
  (params (DeltaSeconds :type Float%20%28single-precision%29))
  (if (not (Variables|Default|GetNewVar_0))
    (Class|Actor|AddActorLocalTransform (Math|Conversions|ToTransform(Vector) "0.000000,0.000000,5.000000") false false)))

(event Game|Damage|EventAnyDamage
  (params (Damage :type Float%20%28single-precision%29) (DamageType :type Damage%20Type%20Object%20Reference) (InstigatedBy :type Controller%20Object%20Reference) (DamageCauser :type Actor%20Object%20Reference))
  (Development|PrintString "Hello"))

(fn ConstructionScript)