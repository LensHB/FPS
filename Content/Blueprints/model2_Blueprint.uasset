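; model2_Blueprint is an actor that alternates between moving its skeletal mesh and standing still.
; While Walk is true, each Tick shifts the mesh one unit along world Y without sweep, resetting its rotation to zero and scale to one.
; A Delay in each branch flips Walk after three seconds, producing a repeating move-and-pause cycle.
; The step ignores delta time, so speed depends on frame rate.
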(event EventBeginPlay)

(event Collision|EventActorBeginOverlap
  (params (OtherActor :type Actor%20Object%20Reference)))

(event EventTick
  (params (DeltaSeconds :type Float%20%28single-precision%29))
  (if (Variables|Default|Getwalk)
    (Transformation|SetWorldTransform (Variables|SkeletalMeshActor|GetSkeletalMeshComponent) (Math|Transform|MakeTransform (+ (Transformation|GetWorldLocation (Variables|SkeletalMeshActor|GetSkeletalMeshComponent)) (Math|Vector|MakeVector 0.0 1.0 0.0))) false false)
    (Utilities|FlowControl|Delay 3.0)
    (Variables|Default|Setwalk false)
    (else
      (Utilities|FlowControl|Delay 3.0)
      (Variables|Default|Setwalk true))))

(fn ConstructionScript)